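; Player character Blueprint with a camera-based check for interactable actors, caching the HUD widget from GM_Base on BeginPlay.
; BPInteractCheck sphere-traces ahead of the camera and stores the hit actor if it implements InteractInterface, otherwise clears it.
; Both outcomes call the HUD's DisplayMessage with false.
; The yaw-relative movement graphs, which call a separate InteractCheck, are disconnected and never run.
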(event EventBeginPlay
  (bind _asgm_base (Utilities|Casting|CastToGM_Base (Game|GetGameMode)))
  (Variables|Default|SetBP_HUD (Variables|/Script/JumpScare.JumpScareGameModeBase|GetHUDWidget _asgm_base)))

(fn ConstructionScript)

(fn BPInteractCheck
  (bind _cameracomponent (Variables|Default|GetCameraComponent))
  (bind _returnvalue (Transformation|GetWorldLocation _cameracomponent))
  (bind _returnvalue_2 (Math|Vector|GetForwardVector _cameracomponent))
  (bind _outhit (Collision|SphereTraceByChannel (+ _returnvalue (* _returnvalue_2 2e+02)) (+ _returnvalue (* _returnvalue_2 5e+02)) 1e+01 "TraceTypeQuery2" false 0 "ForOneFrame"))
  (if (.bblockinghit _outhit)
    (if (Utilities|DoesObjectImplementInterface (.hitactor _outhit) "/Script/JumpScare.InteractInterface")
      (bind _bp_interact_actor (Variables|Default|GetBP_Interact%20Actor)
        (:then
          (if (== _bp_interact_actor (.hitactor _outhit))
            _
            (else
              (Variables|Default|SetBP_Interact%20Actor (.hitactor _outhit) :!label _label))))
        (:else
          (goto _label)))
      (Class|HUDWidget|DisplayMessage (Variables|Default|GetBP_HUD) false)
      (return (Variables|Default|GetBP_Interact%20Actor))
      (else
        _)))
  (Variables|Default|SetBP_Interact%20Actor 0)
  (Class|HUDWidget|DisplayMessage (Variables|Default|GetBP_HUD) false)
  (return (Variables|Default|GetBP_Interact%20Actor)))