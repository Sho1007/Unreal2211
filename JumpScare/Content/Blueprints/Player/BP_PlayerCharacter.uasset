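; Player character Blueprint that handles movement, camera look and interaction with NPCs.
; Movement axis events follow control yaw and also run InteractCheck, a camera-forward sphere trace with debug drawing.
; InteractCheck caches hit actors implementing InteractInterface and calls DisplayMessage on the HUD taken from GM_Base.
; Pressing Interact reruns the check and calls Interact on the result through a BP_NPC cast rather than the interface.
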(event EventBeginPlay
  (bind _asgm_base (Utilities|Casting|CastToGM_Base (Game|GetGameMode)))
  (Variables|Default|SetHUD (Variables|/Script/JumpScare.JumpScareGameModeBase|GetHUDWidget _asgm_base)))

(event Input|ActionEvents|InputActionInteract
  (params (Key :type Key%20Structure :default "None"))
  (:Pressed
    (bind _interactactor (CallFunction|InteractCheck))
    (Utilities|IsValid _interactactor
      (:Is%20Valid
        (bind _asbp_npc (Utilities|Casting|CastToBP_NPC _interactactor))
        (Class|DialogueNPC|Interact _asbp_npc)))))

(event Input|AxisEvents|InputAxisMoveForward
  (params (AxisValue :type Float%20%28single-precision%29))
  (Pawn|Input|AddMovementInput (Math|Vector|GetForwardVector (Math|Rotator|MakeRotator 0.0 0.0 (.yaw (Pawn|GetControlRotation :!class /Script/Engine.Pawn)))) AxisValue false)
  (CallFunction|InteractCheck))

(event Input|AxisEvents|InputAxisMoveRight
  (params (AxisValue :type Float%20%28single-precision%29))
  (Pawn|Input|AddMovementInput (Math|Vector|GetRightVector (Math|Rotator|MakeRotator 0.0 0.0 (.yaw (Pawn|GetControlRotation :!class /Script/Engine.Pawn)))) AxisValue false)
  (CallFunction|InteractCheck))

(event Input|AxisEvents|InputAxisLookUp
  (params (AxisValue :type Float%20%28single-precision%29))
  (Pawn|Input|AddControllerPitchInput AxisValue))

(event Input|AxisEvents|InputAxisLookRight
  (params (AxisValue :type Float%20%28single-precision%29))
  (Pawn|Input|AddControllerYawInput AxisValue))

(fn ConstructionScript)

(fn InteractCheck
  (bind _camera (Variables|Default|GetCamera))
  (bind _returnvalue (Transformation|GetWorldLocation _camera))
  (bind _returnvalue_2 (Math|Vector|GetForwardVector _camera))
  (bind _outhit (Collision|SphereTraceByChannel (+ _returnvalue (* _returnvalue_2 2e+02)) (+ _returnvalue (* _returnvalue_2 5e+02)) 1e+01 "TraceTypeQuery2" false 0 "ForOneFrame"))
  (if (.bblockinghit _outhit)
    (if (Utilities|DoesObjectImplementInterface (.hitactor _outhit) "/Script/JumpScare.InteractInterface")
      (bind _interact_actor (Variables|Default|GetInteract%20Actor)
        (:then
          (if (== _interact_actor (.hitactor _outhit))
            (Class|HUDWidget|DisplayMessage (Variables|Default|GetHUD) false)
            (return (Variables|Default|GetInteract%20Actor))
            (else
              _)))
        (:else
          _))
      (Variables|Default|SetInteract%20Actor (.hitactor _outhit))
      (else
        (Variables|Default|SetInteract%20Actor 0 :!label _label)
        (Class|HUDWidget|DisplayMessage (Variables|Default|GetHUD) false)
        (return (Variables|Default|GetInteract%20Actor))))
    (else
      (goto _label))))